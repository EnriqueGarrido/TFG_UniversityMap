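; Inventory component that holds a fixed number of item slots and toggles an inventory window on the player's HUD canvas.
; BeginPlay sizes the slot array, and OpenClose creates or removes the centered widget, passing itself as the inventory.
; AddInventory tops up non-full stacks of the same class for stackable items, recursing with any overflow.
; Other items fill the first empty slot, and AddInventory always returns true.
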(event EventBeginPlay
  (CallFunction|InitializeInventory))

(fn OpenClose
  (bind _windowinventory (Variables|Default|GetWindowInventory)
    (:then
      (Widget|RemovefromParent _windowinventory)
      (Variables|Default|SetWindowInventory 0))
    (:else
      (bind _returnvalue (UserInterface|CreateWidget "/Game/UniversityGame/Blueprints/Widgets/InventoryWindow.InventoryWindow_C" (Game|GetPlayerController 0) self))
      (Variables|Default|SetWindowInventory _returnvalue)
      (bind _asplayer_controller_university (Utilities|Casting|CastToPlayerControllerUniversity (Game|GetPlayerController 0)))
      (bind _returnvalue_2 (Class|CanvasPanel|AddChildtoCanvas (Variables|/Game/UniversityGame/Blueprints/Widgets/HUDActor.HUDActor_C|GetPanel (Variables|/Game/UniversityGame/Blueprints/PlayerControllerUniversity.PlayerControllerUniversity_C|GetHUDScreen _asplayer_controller_university)) (Variables|Default|GetWindowInventory)))
      (Class|CanvasPanelSlot|SetAutoSize _returnvalue_2 true)
      (Class|CanvasPanelSlot|SetAlignment _returnvalue_2 "(X=0.500000,Y=0.500000)")
      (Class|CanvasPanelSlot|SetAnchors _returnvalue_2 (Utilities|Struct|MakeAnchors "(X=0.500000,Y=0.500000)" "(X=0.500000,Y=0.500000)"))
      (Class|CanvasPanelSlot|SetPosition _returnvalue_2 (Variables|Default|GetPosition)))))

(fn AddInventory
  (params (ContainAdd :type Space%20EST%20Structure))
  (if (.isapilable (.objectstructure ContainAdd))
    (bind _indexapile (Utilities|ApileMacro ContainAdd)
      (:True
        (CallFunction|AddtoPile ContainAdd _indexapile))
      (:False
        (CallFunction|GenerateApile ContainAdd :!label _label)))
    (else
      (goto _label)))
  (return true))

(fn InitializeInventory
  (Utilities|Array|Resize (Variables|Default|GetInventory) (Variables|Default|GetQuantity)))

(fn GenerateApile
  (params (ContainAdd :type Space%20EST%20Structure))
  (bind _inventory (Variables|Default|GetInventory))
  (Utilities|Array|SetArrayElem _inventory (Utilities|Array|FindItem _inventory (Utilities|Struct|MakeSpace_EST "(Name_2_C86DE4FE4674F7E1165864A6FFB9AFCF=NSLOCTEXT(\"[08852F4D4F581E74ABC653943C1D677D]\", \"ADE4D8624A356AA1E53EF6AE52FC3468\", \"Pendrive\"),IsApilable_5_5F8475DD4BCC92DC034CFD9C427F931D=True,Image_8_74A6702C48206007F573E9B2D797650B=None,MaxApilable_11_20AAEE324C7C272C47F88EA60DF864C2=20,Class_19_324369D34472BED732237B93D32EFE85=None)")) ContainAdd))

(fn AddtoPile
  (params (SpaceEST :type Space%20EST%20Structure) (IndexSpace :type Integer))
  (bind _inventory (Variables|Default|GetInventory))
  (bind _inventory_2 (Variables|Default|GetInventory))
  (bind _maxapilable (Utilities|Struct|BreakObject_EST (.objectstructure SpaceEST)))
  (bind _output (Utilities|Array|Get(acopy) _inventory IndexSpace))
  (bind _output_2 (Utilities|Array|Get(acopy) _inventory_2 IndexSpace))
  (bind _output_get (Variables|Default|SetQuantityActual (.quantity _output)))
  (if (> (+ (.Quantity (Utilities|Struct|BreakSpace_EST SpaceEST)) _output_get) (.maxapilable (.objectstructure _output)))
    (Utilities|Array|SetArrayElem (Variables|Default|GetInventory) IndexSpace (Utilities|Struct|MakeSpace_EST (.objectstructure SpaceEST) _maxapilable))
    (CallFunction|AddInventory (Utilities|Struct|MakeSpace_EST (.objectstructure SpaceEST) (- (.quantity SpaceEST) (- _maxapilable (Variables|Default|GetQuantityActual)))))
    (else
      (Utilities|Array|SetArrayElem _inventory_2 IndexSpace (Utilities|Struct|MakeSpace_EST (.objectstructure _output_2) (+ (.quantity SpaceEST) (.quantity _output_2))))))
  (return))