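; Robot enemy that runs the Robot_AC behavior tree and shows a health-bar widget that yaws to face the player.
; A box overlap with the player's tagged capsule sets TouchingYou, which Tick copies to the blackboard while updating the bar.
; When health runs out, Tick ragdolls the mesh and, after a delay, updates MainActor's kills, record, spawn flag and animation mode, then destroys the robot.
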(event OnComponentBeginOverlap(Box)
  (params (OverlappedComponent :type Primitive%20Component%20Object%20Reference) (OtherActor :type Actor%20Object%20Reference) (OtherComp :type Primitive%20Component%20Object%20Reference) (OtherBodyIndex :type Integer) (bFromSweep :type Boolean) (SweepResult :type Hit%20Result%20Structure%20%28by%20ref%29))
  ;[1 1 1] Touching actor
  (if (Components|ComponentHasTag OtherComp "CapsuleActor")
    (Variables|Default|SetTouchingYou true)))

(event OnComponentEndOverlap(Box)
  (params (OverlappedComponent :type Primitive%20Component%20Object%20Reference) (OtherActor :type Actor%20Object%20Reference) (OtherComp :type Primitive%20Component%20Object%20Reference) (OtherBodyIndex :type Integer))
  ;[1 1 1] Touching actor
  (if (Components|ComponentHasTag OtherComp "CapsuleActor")
    (Variables|Default|SetTouchingYou false)
    (Components|Animation|PlayAnimation (Variables|Character|GetMesh) "/Game/UniversityGame/Animations/NaOT/Walking_NaOT.Walking_NaOT" true)))

(event EventBeginPlay
  ;[1 1 1] Health Enemy
  (AI|RunBehaviorTree (AI|GetAIController self) "/Game/UniversityGame/Blueprints/IAEnemy/Robot_AC.Robot_AC"))

(event EventTick
  (params (DeltaSeconds :type Float%20%28single-precision%29))
  (bind _capsulecomponent (Variables|Collision|GetCapsuleComponent))
  (bind _mesh (Variables|Character|GetMesh))
  ;[1 1 1] Health Enemy
  (bind _ashealth_enemy (Utilities|Casting|CastToHealthEnemy (UserInterface|GetUserWidgetObject (Variables|Default|GetHealth))))
  (if (> (Variables|Default|GetHealthenemy) 0.0)
    (Progress|SetPercent (Variables|/Game/UniversityGame/Blueprints/Widgets/HealthEnemy.HealthEnemy_C|GetProgressBar_289 _ashealth_enemy) (/ (Variables|Default|GetHealthenemy) 1e+02))
    (Transformation|SetWorldRotation (Variables|Default|GetHealth) (Math|Rotator|MakeRotator 0.0 0.0 (.Yaw (Math|Rotator|BreakRotator (Math|Rotator|FindLookatRotation (Transformation|GetWorldLocation (Variables|Default|GetHealth)) (Transformation|GetActorLocation (Game|GetPlayerCharacter 0)))))) false false)
    (AI|Components|Blackboard|SetValueasBool (AI|GetBlackboard 0) (Utilities|Name|MakeLiteralName "TouchingYou") (Variables|Default|GetTouchingYou))
    (else
      (Physics|SetSimulatePhysics _capsulecomponent false)
      (Collision|SetCollisionResponsetoChannel _capsulecomponent "ECC_PhysicsBody" "ECR_Ignore")
      (Class|SkeletalMeshComponent|SetAllBodiesBelowSimulatePhysics _mesh (Class|SkinnedMeshComponent|GetBoneName _mesh) true true)
      (Rendering|SetVisibility (Variables|Default|GetHealth) false false)
      (Utilities|FlowControl|Delay 1.0)
      (bind _asmain_actor (Utilities|Casting|CastToMainActor (Game|GetPlayerCharacter 0)))
      (Variables|/Game/UniversityGame/Blueprints/Characters/MainActor.MainActor_C|SetRobotKills _asmain_actor (+ (Variables|/Game/UniversityGame/Blueprints/Characters/MainActor.MainActor_C|GetRobotKills _asmain_actor) 1))
      (Variables|/Game/UniversityGame/Blueprints/Characters/MainActor.MainActor_C|SethasSpawnedRobot _asmain_actor false)
      (Variables|/Game/UniversityGame/Blueprints/Characters/MainActor.MainActor_C|SetRecord _asmain_actor (+ (Variables|/Game/UniversityGame/Blueprints/Characters/MainActor.MainActor_C|GetRecord _asmain_actor) 3))
      (Components|Animation|SetAnimationMode (Variables|/Script/Engine.Character|GetMesh _asmain_actor) "AnimationBlueprint")
      (Actor|DestroyActor))))

(fn ConstructionScript)