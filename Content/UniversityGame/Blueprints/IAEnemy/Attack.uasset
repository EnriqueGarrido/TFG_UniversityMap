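; Behavior tree task that makes a RobotEnemy perform a melee attack on the player.
; It plays one of three random punch, kick or melee animations on the robot's mesh, then waits briefly.
; If the robot's TouchingYou flag is set, it subtracts the MainActor's own DamageReceive, truncated, from that player's Health.
; The task finishes successfully on hit or miss, but never finishes if a cast fails.
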(event EventReceiveExecuteAI
  (params (OwnerController :type AI%20Controller%20Object%20Reference) (ControlledPawn :type Pawn%20Object%20Reference))
  (bind _asrobot_enemy (Utilities|Casting|CastToRobotEnemy ControlledPawn))
  (Components|Animation|PlayAnimation (Variables|/Script/Engine.Character|GetMesh _asrobot_enemy) (Utilities|Select :Index (Math|Random|RandomInteger 3) :Option%200 "/Game/UniversityGame/Animations/NaOT/Punch_NaOT.Punch_NaOT" :Option%201 "/Game/UniversityGame/Animations/NaOT/Kicking_NaOT.Kicking_NaOT" :Option%202 "/Game/UniversityGame/Animations/NaOT/Melee_NaOT.Melee_NaOT") false)
  (Utilities|FlowControl|Delay 0.4)
  (if (Variables|/Game/UniversityGame/Blueprints/IAEnemy/RobotEnemy.RobotEnemy_C|GetTouchingYou _asrobot_enemy)
    (bind _asmain_actor (Utilities|Casting|CastToMainActor (Game|GetPlayerCharacter 0)))
    (Variables|/Game/UniversityGame/Blueprints/Characters/MainActor.MainActor_C|SetHealth _asmain_actor (- (Variables|/Game/UniversityGame/Blueprints/Characters/MainActor.MainActor_C|GetHealth _asmain_actor) (Math|Float|Truncate (Variables|/Game/UniversityGame/Blueprints/Characters/MainActor.MainActor_C|GetDamageReceive _asmain_actor)))))
  (AI|BehaviorTree|FinishExecute true))