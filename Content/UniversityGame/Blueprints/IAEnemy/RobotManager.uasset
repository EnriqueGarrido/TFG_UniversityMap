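; RobotManager is a robot wave spawner that reads and updates state on the player's MainActor, cached at BeginPlay.
; GenerateEnemies spawns three RobotEnemy AIs with the Robot_AC behavior tree at preset locations and increments the wave count.
; Disconnected logic would trigger a wave when the kill count is a multiple of three, then adjust attack, damage received and robot speed within limits.
; Tick is empty, so nothing here calls GenerateEnemies.
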(event EventTick
  (params (DeltaSeconds :type Float%20%28single-precision%29))
  ;[1 1 1] Interaction with Robots
)

(event Collision|EventActorBeginOverlap
  (params (OtherActor :type Actor%20Object%20Reference)))

(event EventBeginPlay
  (bind _asmain_actor (Utilities|Casting|CastToMainActor (Game|GetPlayerCharacter 0)))
  (Variables|Default|SetMainActor _asmain_actor))

(fn ConstructionScript)

(fn GenerateEnemies
  (bind _mainactor (Variables|Default|GetMainActor))
  (for _index (range 0 2)
    (AI|SpawnAIFromClass "/Game/UniversityGame/Blueprints/IAEnemy/RobotEnemy.RobotEnemy_C" "/Game/UniversityGame/Blueprints/IAEnemy/Robot_AC.Robot_AC" (Utilities|Array|Get(acopy) (Variables|Default|GetLocation) _index) "0, 0, 0" false))
  (Variables|/Game/UniversityGame/Blueprints/Characters/MainActor.MainActor_C|SetnumWaves _mainactor (+ (Variables|/Game/UniversityGame/Blueprints/Characters/MainActor.MainActor_C|GetnumWaves _mainactor) 1)))