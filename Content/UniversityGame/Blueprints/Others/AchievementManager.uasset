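; Achievement manager for the university game that unlocks two achievements: finding the hidden objects and talking to all characters.
; On BeginPlay it caches the GameInstanceUniversity, then polls that instance's HiddenObjects and PeopleTalk counters every Tick against hardcoded totals.
; When a counter matches, it shows an AchievementWidget with Spanish text on the player screen for a short delay.
; Local boolean flags make each popup fire only once.
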(event EventTick
  (params (DeltaSeconds :type Float%20%28single-precision%29))
  (bind _returnvalue (Game|GetPlayerController 0))
  (bind _gameinstance (Variables|Default|GetGameInstance))
  (Utilities|FlowControl|Sequence
    (:then_0
      (if (not (Variables|Default|GetAchieve1))
        (if (== (Variables|/Game/UniversityGame/Blueprints/GameInstanceUniversity.GameInstanceUniversity_C|GetHiddenObjects _gameinstance) 3)
          (bind _returnvalue_2 (UserInterface|CreateWidget "/Game/UniversityGame/Blueprints/Widgets/AchievementWidget.AchievementWidget_C" _returnvalue "Encuentra los 3 objetos ocultos"))
          (UserInterface|Viewport|AddtoPlayerScreen _returnvalue_2)
          (Variables|Default|SetAchieve1 true)
          (Utilities|FlowControl|Delay 2.0)
          (Widget|RemovefromParent _returnvalue_2))))
    (:then_1
      (if (not (Variables|Default|GetAchieve2))
        (if (== (Variables|/Game/UniversityGame/Blueprints/GameInstanceUniversity.GameInstanceUniversity_C|GetpeopleTalk _gameinstance) 25)
          (bind _returnvalue_3 (UserInterface|CreateWidget "/Game/UniversityGame/Blueprints/Widgets/AchievementWidget.AchievementWidget_C" _returnvalue "Habla con todos los personajes"))
          (UserInterface|Viewport|AddtoPlayerScreen _returnvalue_3)
          (Variables|Default|SetAchieve2 true)
          (Utilities|FlowControl|Delay 2.0)
          (Widget|RemovefromParent _returnvalue_3))))))

(event EventBeginPlay
  (bind _asgame_instance_university (Utilities|Casting|CastToGameInstanceUniversity (Game|GetGameInstance)))
  (Variables|Default|SetGameInstance _asgame_instance_university))

(fn ConstructionScript)