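; ActorParent is an actor Blueprint, by its name a base class, that reveals a prompt and accepts input while something overlaps its Box.
; Its TextRender and Cube components start hidden on BeginPlay.
; Box begin overlap shows both and enables input for player controller 0, and end overlap hides them and disables that input.
; The overlap events do not filter which actor triggers them.
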(event OnComponentBeginOverlap(Box)
  (params (OverlappedComponent :type Primitive%20Component%20Object%20Reference) (OtherActor :type Actor%20Object%20Reference) (OtherComp :type Primitive%20Component%20Object%20Reference) (OtherBodyIndex :type Integer) (bFromSweep :type Boolean) (SweepResult :type Hit%20Result%20Structure%20%28by%20ref%29))
  ;[1 1 1] Appear or dessapear the colission box
  (Rendering|SetVisibility (Variables|Default|GetTextRender) true false)
  (Input|EnableInput 0)
  (Input|EnableInput (Game|GetPlayerController 0)))

(event OnComponentEndOverlap(Box)
  (params (OverlappedComponent :type Primitive%20Component%20Object%20Reference) (OtherActor :type Actor%20Object%20Reference) (OtherComp :type Primitive%20Component%20Object%20Reference) (OtherBodyIndex :type Integer))
  ;[1 1 1] Appear or dessapear the colission box
  (Rendering|SetVisibility (Variables|Default|GetTextRender) false false)
  (Input|DisableInput (Game|GetPlayerController 0)))

(event EventBeginPlay
  ;[1 1 1] Appear or dessapear the colission box
  (Rendering|SetVisibility (Variables|Default|GetTextRender) false false))

(fn ConstructionScript)