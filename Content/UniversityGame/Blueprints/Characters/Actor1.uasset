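; Actor1 is a teacher NPC that starts a dialogue when the Talk input is pressed.
; It hides its text prompt and picks one of three dialogue widgets from the StateTeacher enum: not-turn, turn or mission.
; It then shows the cursor, switches to UI-only input, moves the view to the CameraActor tagged CameraNPC_1 and flags the MainActor's HUD as unavailable.
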(event EventBeginPlay
  (|CallParentFunction))

(event Input|ActionEvents|InputActionTalk
  (params (Key :type Key%20Structure))
  (bind _returnvalue (Game|GetPlayerController 0))
  (bind _stateteacher (Variables|Default|GetStateTeacher))
  ;[1 1 1] Inicio de diálogo
  (:Pressed
    (Rendering|SetVisibility (Variables|Default|GetTextRender) false false)
    (if (Utilities|Enum|Equal(Enum) _stateteacher "NewEnumerator0")
      (bind _returnvalue_2 (UserInterface|CreateWidget "/Game/UniversityGame/Blueprints/Dialogues/Dialogue_1/Dialogue_NotTurn_1.Dialogue_NotTurn_1_C" _returnvalue))
      (UserInterface|Viewport|AddtoPlayerScreen _returnvalue_2)
      (Variables|/Script/Engine.PlayerController|SetbShowMouseCursor _returnvalue true :!label _label)
      (Input|SetInputModeUIOnly _returnvalue 0 "DoNotLock")
      (bind _outactors (Actor|GetAllActorsOfClass "/Script/Engine.CameraActor"))
      (for _array_element _outactors
        (if (Actor|ActorHasTag _array_element "CameraNPC_1")
          (Game|Player|SetViewTargetwithBlend (Game|GetPlayerController 0) _array_element 0.0 "VTBlend_Linear" 0.0 false)
          (bind _asmain_actor (Utilities|Casting|CastToMainActor (Game|GetPlayerCharacter 0)))
          (Variables|/Game/UniversityGame/Blueprints/Characters/MainActor.MainActor_C|SetHUDAviable _asmain_actor false)))
      (elif (Utilities|Enum|Equal(Enum) _stateteacher "NewEnumerator1")
        (bind _returnvalue_3 (UserInterface|CreateWidget "/Game/UniversityGame/Blueprints/Dialogues/Dialogue_1/Dialogue_Turn_1.Dialogue_Turn_1_C" _returnvalue))
        (UserInterface|Viewport|AddtoPlayerScreen _returnvalue_3)
        (goto _label)
        (elif (Utilities|Enum|Equal(Enum) _stateteacher "NewEnumerator2")
          (bind _returnvalue_4 (UserInterface|CreateWidget "/Game/UniversityGame/Blueprints/Dialogues/Dialogue_1/Dialogue_Mission_1.Dialogue_Mission_1_C" _returnvalue))
          (UserInterface|Viewport|AddtoPlayerScreen _returnvalue_4)
          (goto _label))))))

(fn ConstructionScript
  (|CallParentFunction))