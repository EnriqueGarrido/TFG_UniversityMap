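; Student NPC Cristian, a child Blueprint that the player can talk to and record in the people collection.
; The Talk input hides the prompt, opens his dialogue widget in UI-only mode, blends to the camera tagged CameraCristian and flags the MainActor HUD unavailable.
; The first talk also hides the marker meshes, increments the GameInstance talk count, saves his collection entry to the save slot and calls IncrementRecord.
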(event EventBeginPlay
  (|CallParentFunction))

(event Input|ActionEvents|InputActionTalk
  (params (Key :type Key%20Structure))
  (bind _returnvalue (Game|GetPlayerController 0))
  ;[1 1 1] Talk with Cristian
  (:Pressed
    (Rendering|SetVisibility (Variables|Default|GetTextRender) false false)
    (bind _returnvalue_2 (UserInterface|CreateWidget "/Game/UniversityGame/Blueprints/Dialogues/Dialogue_Cristian/Dialogue_1_Cristian.Dialogue_1_Cristian_C" _returnvalue))
    (UserInterface|Viewport|AddtoPlayerScreen _returnvalue_2)
    (Variables|/Script/Engine.PlayerController|SetbShowMouseCursor _returnvalue true)
    (Input|SetInputModeUIOnly _returnvalue 0 "DoNotLock")
    (bind _outactors (Actor|GetAllActorsOfClass "/Script/Engine.CameraActor"))
    (for _array_element _outactors
      (if (Actor|ActorHasTag _array_element "CameraCristian")
        (Game|Player|SetViewTargetwithBlend (Game|GetPlayerController 0) _array_element 0.0 "VTBlend_Linear" 0.0 false)
        (bind _asmain_actor (Utilities|Casting|CastToMainActor (Game|GetPlayerCharacter 0)))
        (Variables|/Game/UniversityGame/Blueprints/Characters/MainActor.MainActor_C|SetHUDAviable _asmain_actor false)
        (if (not (Variables|Default|GethasTalk))
          (Utilities|Casting|CastToMainActor (Game|GetPlayerCharacter 0))
          (if (not (Variables|Default|GethasTalk))
            (Math|Integer|IncrementInt (Variables|/Game/UniversityGame/Blueprints/GameInstanceUniversity.GameInstanceUniversity_C|GetpeopleTalk (Variables|Default|GetGameInstance))
              (:%20%20
                (Variables|Default|SethasTalk true)
                (Rendering|SetVisibility (Variables|Default|GetCylinder) false false)
                (bind _returnvalue_3 (SaveGame|LoadGamefromSlot "Ranura1"))
                (bind _asgame_saved (Utilities|Casting|CastToGameSaved _returnvalue_3))
                (bind _output_get (Variables|Default|SetGameSaved _asgame_saved))
                (Utilities|Array|SetArrayElem (Variables|/Game/UniversityGame/Blueprints/GameSaved.GameSaved_C|GetPeopleCollections _output_get) 16 (Utilities|Struct|MakeCollection_EST "/Game/UniversityGame/Images/Characters/Estudiante_Cristian.Estudiante_Cristian" "Cristian" "Estudiante" true))
                (SaveGame|SaveGametoSlot _output_get "Ranura1")
                (CallFunction|IncrementRecord)))))))))

(fn ConstructionScript
  (|CallParentFunction))