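; Charo is a talkable NPC actor from the Consejería who opens one of three dialogue widgets based on StateTeacher when Talk is pressed.
; Talking hides the prompt, switches to UI-only input, blends to the camera tagged "CameraCharo" and flags the player's HUD unavailable.
; The first talk also increments the GameInstance talk count, saves Charo into the people collection and calls IncrementRecord.
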(event EventBeginPlay
  (|CallParentFunction))

(event Input|ActionEvents|InputActionTalk
  (params (Key :type Key%20Structure))
  (bind _returnvalue (Game|GetPlayerController 0))
  (bind _stateteacher (Variables|Default|GetStateTeacher))
  ;[1 1 1] Talk with Charo
  (:Pressed
    (Rendering|SetVisibility (Variables|Default|GetTextRender) false false)
    (if (Utilities|Enum|Equal(Enum) _stateteacher "NewEnumerator0")
      (bind _returnvalue_2 (UserInterface|CreateWidget "/Game/UniversityGame/Blueprints/Dialogues/Dialogue_Charo/Dialogue_1_Charo.Dialogue_1_Charo_C" _returnvalue))
      (UserInterface|Viewport|AddtoPlayerScreen _returnvalue_2)
      (Variables|/Script/Engine.PlayerController|SetbShowMouseCursor _returnvalue true :!label _label)
      (Input|DisableInput (Game|GetPlayerCharacter 0) (Game|GetPlayerController 0))
      (Input|SetInputModeUIOnly _returnvalue 0 "DoNotLock")
      (bind _outactors (Actor|GetAllActorsOfClass "/Script/Engine.CameraActor"))
      (for _array_element _outactors
        (if (Actor|ActorHasTag _array_element "CameraCharo")
          (Game|Player|SetViewTargetwithBlend (Game|GetPlayerController 0) _array_element 0.0 "VTBlend_Linear" 0.0 false)
          (bind _asmain_actor (Utilities|Casting|CastToMainActor (Game|GetPlayerCharacter 0)))
          (Variables|/Game/UniversityGame/Blueprints/Characters/MainActor.MainActor_C|SetHUDAviable _asmain_actor false)
          (if (not (Variables|Default|GethasTalk))
            (Math|Integer|IncrementInt (Variables|/Game/UniversityGame/Blueprints/GameInstanceUniversity.GameInstanceUniversity_C|GetpeopleTalk (Variables|Default|GetGameInstance))
              (:%20%20
                (Variables|Default|SethasTalk true)
                (bind _returnvalue_3 (SaveGame|LoadGamefromSlot "Ranura1"))
                (bind _asgame_saved (Utilities|Casting|CastToGameSaved _returnvalue_3))
                (bind _output_get (Variables|Default|SetGameSaved _asgame_saved))
                (Utilities|Array|SetArrayElem (Variables|/Game/UniversityGame/Blueprints/GameSaved.GameSaved_C|GetPeopleCollections _output_get) 1 (Utilities|Struct|MakeCollection_EST "/Game/UniversityGame/Images/Characters/Consejeria_Charo.Consejeria_Charo" "Charo" "Consejería" true))
                (SaveGame|SaveGametoSlot _output_get "Ranura1")
                (CallFunction|IncrementRecord))))))
      (elif (Utilities|Enum|Equal(Enum) _stateteacher "NewEnumerator1")
        (bind _returnvalue_4 (UserInterface|CreateWidget "/Game/UniversityGame/Blueprints/Dialogues/Dialogue_Charo/Dialogue_2_Charo.Dialogue_2_Charo_C" _returnvalue))
        (UserInterface|Viewport|AddtoPlayerScreen _returnvalue_4)
        (goto _label)
        (elif (Utilities|Enum|Equal(Enum) _stateteacher "NewEnumerator2")
          (bind _returnvalue_5 (UserInterface|CreateWidget "/Game/UniversityGame/Blueprints/Dialogues/Dialogue_Charo/Dialogue_3_Charo.Dialogue_3_Charo_C"))
          (UserInterface|Viewport|AddtoPlayerScreen _returnvalue_5)
          (goto _label))))))

(fn ConstructionScript
  (|CallParentFunction))