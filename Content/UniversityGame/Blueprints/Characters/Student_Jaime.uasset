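; Jaime, a student NPC in the university game who opens a dialogue when the Talk input is pressed.
; StateTeacher selects one of two dialogue widgets, then input switches to UI-only and the view moves to the camera tagged CameraJaime.
; It also hides the NPC's text and mesh components and turns off the player's HUD flag.
; The first talk increments PeopleTalk, saves Jaime into the people collection in slot Ranura1 and calls IncrementRecord.
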(event EventBeginPlay
  (|CallParentFunction) ; This node is disabled and will not be called.\nDrag off pins to build functionality.
)

(event Collision|EventActorBeginOverlap
  (params (OtherActor :type Actor%20Object%20Reference)))

(event EventTick
  (params (DeltaSeconds :type Float%20%28single-precision%29)))

(event Input|ActionEvents|InputActionTalk
  (params (Key :type Key%20Structure))
  (bind _returnvalue (Game|GetPlayerController 0))
  (bind _stateteacher (Variables|Default|GetStateTeacher))
  ;[1 1 1] Talk with Jaime
  (:Pressed
    (Rendering|SetVisibility (Variables|Default|GetTextRender) false false)
    (if (Utilities|Enum|Equal(Enum) _stateteacher "NewEnumerator0")
      (bind _returnvalue_2 (UserInterface|CreateWidget "/Game/UniversityGame/Blueprints/Dialogues/Dialogue_Jaime/Dialogue_1_Jaime.Dialogue_1_Jaime_C" _returnvalue))
      (UserInterface|Viewport|AddtoPlayerScreen _returnvalue_2)
      (Variables|/Script/Engine.PlayerController|SetbShowMouseCursor _returnvalue true :!label _label)
      (Input|SetInputModeUIOnly _returnvalue 0 "DoNotLock")
      (Input|DisableInput (Game|GetPlayerCharacter 0) (Game|GetPlayerController 0))
      (bind _outactors (Actor|GetAllActorsOfClass "/Script/Engine.CameraActor"))
      (for _array_element _outactors
        (if (Actor|ActorHasTag _array_element "CameraJaime")
          (Game|Player|SetViewTargetwithBlend (Game|GetPlayerController 0) _array_element 0.0 "VTBlend_Linear" 0.0 false)
          (bind _asmain_actor (Utilities|Casting|CastToMainActor (Game|GetPlayerCharacter 0)))
          (Variables|/Game/UniversityGame/Blueprints/Characters/MainActor.MainActor_C|SetHUDAviable _asmain_actor false)
          (if (not (Variables|Default|GethasTalk))
            (Math|Integer|IncrementInt (Variables|/Game/UniversityGame/Blueprints/GameInstanceUniversity.GameInstanceUniversity_C|GetpeopleTalk (Variables|Default|GetGameInstance))
              (:%20%20
                (Variables|Default|SethasTalk true)
                (bind _returnvalue_3 (SaveGame|LoadGamefromSlot "Ranura1"))
                (bind _asgame_save_university (Utilities|Casting|CastToGameSaveUniversity _returnvalue_3))
                (bind _output_get (Variables|Default|SetGameSaved _asgame_save_university))
                (Utilities|Array|SetArrayElem (Variables|/Game/UniversityGame/Blueprints/GameSaveUniversity.GameSaveUniversity_C|GetPeopleCollections _output_get) 17 (Utilities|Struct|MakeCollection_EST "/Game/UniversityGame/Images/Characters/Estudiante_Jaime.Estudiante_Jaime" "Jaime" "Estudiante 
Trabaja en cirebits" true))
                (SaveGame|SaveGametoSlot _output_get "Ranura1")
                (CallFunction|IncrementRecord))))))
      (elif (Utilities|Enum|Equal(Enum) _stateteacher "NewEnumerator1")
        (bind _returnvalue_4 (UserInterface|CreateWidget "/Game/UniversityGame/Blueprints/Dialogues/Dialogue_Jaime/Dialogue_2_Jaime.Dialogue_2_Jaime_C" _returnvalue))
        (UserInterface|Viewport|AddtoPlayerScreen _returnvalue_4)
        (goto _label)))))

(fn ConstructionScript
  (|CallParentFunction))