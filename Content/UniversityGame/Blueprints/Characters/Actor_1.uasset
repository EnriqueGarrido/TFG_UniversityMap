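; Actor_1 is an interaction actor, apparently for an NPC, that starts a dialogue when the player presses Talk.
; A box overlap shows a text prompt and enables input on the actor, and leaving the box hides the prompt and disables input.
; Talk hides the prompt, opens the Dialogue_1 widget in UI-only input with the cursor shown, and blends the view to the camera tagged CameraNPC_1.
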(event OnComponentBeginOverlap(Box)
  (params (OverlappedComponent :type Primitive%20Component%20Object%20Reference) (OtherActor :type Actor%20Object%20Reference) (OtherComp :type Primitive%20Component%20Object%20Reference) (OtherBodyIndex :type Integer) (bFromSweep :type Boolean) (SweepResult :type Hit%20Result%20Structure%20%28by%20ref%29))
  ;[1 1 1] Appear or dessapear the colission box
  (Rendering|SetVisibility (Variables|Default|GetTextRender) true false)
  (Input|EnableInput 0)
  (Input|EnableInput (Game|GetPlayerController 0)))

(event OnComponentEndOverlap(Box)
  (params (OverlappedComponent :type Primitive%20Component%20Object%20Reference) (OtherActor :type Actor%20Object%20Reference) (OtherComp :type Primitive%20Component%20Object%20Reference) (OtherBodyIndex :type Integer))
  ;[1 1 1] Appear or dessapear the colission box
  (Rendering|SetVisibility (Variables|Default|GetTextRender) false false)
  (Input|DisableInput (Game|GetPlayerController 0)))

(event EventBeginPlay
  ;[1 1 1] Appear or dessapear the colission box
  (Rendering|SetVisibility (Variables|Default|GetTextRender) false false))

(event Input|ActionEvents|InputActionTalk
  (params (Key :type Key%20Structure))
  (bind _returnvalue (Game|GetPlayerController 0))
  ;[1 1 1] Inicio de diálogo
  (:Pressed
    (Rendering|SetVisibility (Variables|Default|GetTextRender) false false)
    (bind _returnvalue_2 (UserInterface|CreateWidget "/Game/UniversityGame/Blueprints/Dialogues/Dialogue_1.Dialogue_1_C" _returnvalue))
    (UserInterface|Viewport|AddtoPlayerScreen _returnvalue_2)
    (Variables|/Script/Engine.PlayerController|SetbShowMouseCursor _returnvalue true)
    (Input|SetInputModeUIOnly _returnvalue 0 "DoNotLock")
    (bind _outactors (Actor|GetAllActorsOfClass "/Script/Engine.CameraActor"))
    (for _array_element _outactors
      (if (Actor|ActorHasTag _array_element "CameraNPC_1")
        (Game|Player|SetViewTargetwithBlend (Game|GetPlayerController 0) _array_element 0.0 "VTBlend_Linear" 0.0 false)))))

(fn ConstructionScript)