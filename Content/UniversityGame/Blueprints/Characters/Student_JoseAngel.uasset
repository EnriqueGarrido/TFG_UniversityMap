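; Student NPC Blueprint for Jose Angel that the player talks to through the Talk input action.
; Pressing Talk hides its prompt text and cube, opens the Dialogue_1_JoseAngel widget and switches to UI-only input with a visible cursor.
; It then switches the view to the CameraActor tagged CameraJose, clears MainActor's HUDAviable flag and increments its PeopleTalk counter once, guarded by HasTalk.
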(event EventBeginPlay
  (|CallParentFunction))

(event Input|ActionEvents|InputActionTalk
  (params (Key :type Key%20Structure))
  (bind _returnvalue (Game|GetPlayerController 0))
  ;[1 1 1] Talk with JoseAngel
  (:Pressed
    (Rendering|SetVisibility (Variables|Default|GetTextRender) false false)
    (bind _returnvalue_2 (UserInterface|CreateWidget "/Game/UniversityGame/Blueprints/Dialogues/Dialogue_JoseAngel/Dialogue_1_JoseAngel.Dialogue_1_JoseAngel_C" _returnvalue))
    (UserInterface|Viewport|AddtoPlayerScreen _returnvalue_2)
    (Variables|/Script/Engine.PlayerController|SetbShowMouseCursor _returnvalue true)
    (Input|SetInputModeUIOnly _returnvalue 0 "DoNotLock")
    (bind _outactors (Actor|GetAllActorsOfClass "/Script/Engine.CameraActor"))
    (for _array_element _outactors
      (if (Actor|ActorHasTag _array_element "CameraJose")
        (Game|Player|SetViewTargetwithBlend (Game|GetPlayerController 0) _array_element 0.0 "VTBlend_Linear" 0.0 false)
        (bind _asmain_actor (Utilities|Casting|CastToMainActor (Game|GetPlayerCharacter 0)))
        (Variables|/Game/UniversityGame/Blueprints/Characters/MainActor.MainActor_C|SetHUDAviable _asmain_actor false)
        (if (not (Variables|Default|GethasTalk))
          (bind _asmain_actor_2 (Utilities|Casting|CastToMainActor (Game|GetPlayerCharacter 0)))
          (if (not (Variables|Default|GethasTalk))
            (Math|Integer|IncrementInt (Variables|/Game/UniversityGame/Blueprints/Characters/MainActor.MainActor_C|GetpeopleTalk _asmain_actor_2)
              (:%20%20
                (Variables|Default|SethasTalk true)))))))))

(fn ConstructionScript
  (|CallParentFunction))