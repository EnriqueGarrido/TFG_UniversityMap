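; RobotEnemy is an enemy character that shows a floating health bar and dies when its health runs out.
; Every Tick sets the widget's progress bar from the Healthenemy value and yaws it toward the player character.
; At zero health it ragdolls the mesh, hides the bar and destroys itself after a delay.
; Chase logic using AIMoveTo toward MainActor exists but is unconnected, leaving the PawnSensing event empty.
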(event OnSeePawn(PawnSensing)
  (params (Pawn :type Pawn%20Object%20Reference))
  ;[1 1 1] Movement Enemy
)

(event EventBeginPlay
  ;[1 1 1] Health Enemy
)

(event Collision|EventActorBeginOverlap
  (params (OtherActor :type Actor%20Object%20Reference))
  ;[1 1 1] Health Enemy
)

(event EventTick
  (params (DeltaSeconds :type Float%20%28single-precision%29))
  (bind _capsulecomponent (Variables|Collision|GetCapsuleComponent))
  (bind _mesh (Variables|Character|GetMesh))
  ;[1 1 1] Health Enemy
  (bind _ashealth_enemy (Utilities|Casting|CastToHealthEnemy (UserInterface|GetUserWidgetObject (Variables|Default|GetHealth))))
  (if (> (Variables|Default|GetHealthenemy) 0.0)
    (Progress|SetPercent (Variables|/Game/UniversityGame/Blueprints/Widgets/HealthEnemy.HealthEnemy_C|GetProgressBar_289 _ashealth_enemy) (/ (Variables|Default|GetHealthenemy) 1e+02))
    (Transformation|SetWorldRotation (Variables|Default|GetHealth) (Math|Rotator|MakeRotator 0.0 0.0 (.Yaw (Math|Rotator|BreakRotator (Math|Rotator|FindLookatRotation (Transformation|GetWorldLocation (Variables|Default|GetHealth)) (Transformation|GetActorLocation (Game|GetPlayerCharacter 0)))))) false false)
    (else
      (Physics|SetSimulatePhysics _capsulecomponent false)
      (Collision|SetCollisionResponsetoChannel _capsulecomponent "ECC_PhysicsBody" "ECR_Ignore")
      (Class|SkeletalMeshComponent|SetAllBodiesBelowSimulatePhysics _mesh (Class|SkinnedMeshComponent|GetBoneName _mesh) true true)
      (Rendering|SetVisibility (Variables|Default|GetHealth) false false)
      (Utilities|FlowControl|Delay 3.0)
      (Actor|DestroyActor))))

(fn ConstructionScript)