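; NormalDoor is an interactable door actor that the player opens and closes with the OpenDoor input action.
; A Box trigger shows two text prompts and enables player input on begin overlap, then hides them and disables input on end overlap.
; Pressing the action toggles between the rotation saved at BeginPlay and that rotation yawed by a quarter turn, snapping instantly with no animation.
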(event OnComponentBeginOverlap(Box)
  (params (OverlappedComponent :type Primitive%20Component%20Object%20Reference) (OtherActor :type Actor%20Object%20Reference) (OtherComp :type Primitive%20Component%20Object%20Reference) (OtherBodyIndex :type Integer) (bFromSweep :type Boolean) (SweepResult :type Hit%20Result%20Structure%20%28by%20ref%29))
  ;[1 1 1] Appear or desappear the colission box
  (Rendering|SetVisibility (Variables|Default|GetTextRender) true false)
  (Input|EnableInput (Game|GetPlayerController 0)))

(event OnComponentEndOverlap(Box)
  (params (OverlappedComponent :type Primitive%20Component%20Object%20Reference) (OtherActor :type Actor%20Object%20Reference) (OtherComp :type Primitive%20Component%20Object%20Reference) (OtherBodyIndex :type Integer))
  ;[1 1 1] Appear or desappear the colission box
  (Rendering|SetVisibility (Variables|Default|GetTextRender) false false)
  (Input|DisableInput (Game|GetPlayerController 0)))

(event EventBeginPlay
  ;[1 1 1] Event BeginPlay
  (Rendering|SetVisibility (Variables|Default|GetTextRender) false false)
  (Variables|Default|SetRotation (Transformation|GetActorRotation)))

(event Input|ActionEvents|InputActionOpenDoor
  (params (Key :type Key%20Structure))
  (bind _rotation (Variables|Default|GetRotation))
  (bind (_roll _pitch _yaw) (Math|Rotator|BreakRotator _rotation))
  (:Pressed
    ;[1 1 1] Open/Close door
    (if (Variables|Default|GetDoorOpen)
      (Transformation|SetActorRotation (Variables|Default|GetRotation))
      (Variables|Default|SetDoorOpen false)
      (else
        (Transformation|SetActorRotation (Math|Rotator|MakeRotator _roll _pitch (- _yaw 9e+01)))
        (Variables|Default|SetDoorOpen true)))))

(fn ConstructionScript)