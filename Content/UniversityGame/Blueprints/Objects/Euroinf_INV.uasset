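; Hidden collectible actor for the EURO-INF quality seal in a university game, revealed when its box is overlapped.
; The overlap destroys the box, hides the mesh, increments the hidden-object record and the GameInstance counter, and shows a two-second discovery banner.
; It also opens an information widget with an image and Spanish text about the seal, disabling player input and switching to UI-only mode with a visible cursor.
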(event OnComponentBeginOverlap(Box)
  (params (OverlappedComponent :type Primitive%20Component%20Object%20Reference) (OtherActor :type Actor%20Object%20Reference) (OtherComp :type Primitive%20Component%20Object%20Reference) (OtherBodyIndex :type Integer) (bFromSweep :type Boolean) (SweepResult :type Hit%20Result%20Structure%20%28by%20ref%29))
  (bind _returnvalue (Game|GetPlayerController 0))
  ;[1 1 1] You have a pendrive
  (Components|DestroyComponent (Variables|Default|GetBox))
  (bind _asmain_actor (Utilities|Casting|CastToMainActor (Game|GetPlayerCharacter 0)))
  (Variables|/Game/UniversityGame/Blueprints/Characters/MainActor.MainActor_C|SetBanner _asmain_actor "¡Has encontradoel sello- EuroInf!")
  (bind _returnvalue_2 (UserInterface|CreateWidget "/Game/UniversityGame/Blueprints/Widgets/Banner.Banner_C" (Game|GetPlayerController 0)))
  (UserInterface|Viewport|AddtoPlayerScreen _returnvalue_2)
  (Rendering|SetVisibility (Variables|Default|GetStaticMesh) false false)
  (CallFunction|IncrementRecordOculto)
  (bind _returnvalue_3 (UserInterface|CreateWidget "/Game/UniversityGame/Blueprints/Widgets/InformationObjects.InformationObjects_C" 0 (Utilities|Struct|MakeSlateBrush "(X=300.000000,Y=300.000000)" "(Left=0.000000,Top=0.000000,Right=0.000000,Bottom=0.000000)" "(SpecifiedColor=(R=1.000000,G=1.000000,B=1.000000,A=1.000000),ColorUseRule=UseColor_Specified)" "/Game/UniversityGame/Images/CapturaEuroing.CapturaEuroing" "Image" "NoTile" "NoMirror") "La ESI cuenta con el sello internacional de  
excelencia EURO-INF en el Grado de Ingeniería  
Informática. Reconoce que los estudios cumplen  
ampliamente los Estándares de calidad para  
el desarrollo académico y profesional en  
el ámbito de la Informática. Los alumnos  
garantizarán que su formación es de calidad."))
  (UserInterface|Viewport|AddtoPlayerScreen _returnvalue_3)
  (Input|DisableInput (Game|GetPlayerCharacter 0) _returnvalue)
  (Input|SetInputModeUIOnly _returnvalue 0 "DoNotLock")
  (Variables|/Script/Engine.PlayerController|SetbShowMouseCursor _returnvalue true)
  (bind _asgame_instance_university (Utilities|Casting|CastToGameInstanceUniversity (Game|GetGameInstance)))
  (Math|Integer|IncrementInt (Variables|/Game/UniversityGame/Blueprints/GameInstanceUniversity.GameInstanceUniversity_C|GetHiddenObjects _asgame_instance_university)
    (:%20%20
      (Utilities|FlowControl|Delay 2.0)
      (Widget|RemovefromParent _returnvalue_2))))

(event Collision|EventActorBeginOverlap
  (params (OtherActor :type Actor%20Object%20Reference)))

(event EventTick
  (params (DeltaSeconds :type Float%20%28single-precision%29)))

(event EventBeginPlay)

(fn ConstructionScript
  (|CallParentFunction))