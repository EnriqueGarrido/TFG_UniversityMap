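; Certificate pickup that the player finds by overlapping its Box trigger, built on a parent class whose UseObject it leaves unchanged.
; The first overlap by any actor destroys the Box, sets MainActor's found-certificate message and shows a Banner widget.
; It also reveals every Actor_Eduardo's Cylinder and Sphere, changes their StateTeacher and calls IncrementRecord.
; The mesh hides immediately, then a short delay removes the banner and destroys the actor.
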(event OnComponentBeginOverlap(Box)
  (params (OverlappedComponent :type Primitive%20Component%20Object%20Reference) (OtherActor :type Actor%20Object%20Reference) (OtherComp :type Primitive%20Component%20Object%20Reference) (OtherBodyIndex :type Integer) (bFromSweep :type Boolean) (SweepResult :type Hit%20Result%20Structure%20%28by%20ref%29))
  (Components|DestroyComponent (Variables|Default|GetBox))
  (bind _asmain_actor (Utilities|Casting|CastToMainActor (Game|GetPlayerCharacter 0)))
  (Variables|/Game/UniversityGame/Blueprints/Characters/MainActor.MainActor_C|SetBanner _asmain_actor "¡Has encontrado el certificado!")
  (bind _returnvalue (UserInterface|CreateWidget "/Game/UniversityGame/Blueprints/Widgets/Banner.Banner_C" (Game|GetPlayerController 0)))
  (bind _outactors (Actor|GetAllActorsOfClass "/Game/UniversityGame/Blueprints/Characters/Actor_Eduardo.Actor_Eduardo_C"))
  (for _array_element _outactors
    (Rendering|SetVisibility (Variables|/Game/UniversityGame/Blueprints/Characters/ActorParent.ActorParent_C|GetCylinder _array_element) true false)
    (Variables|/Game/UniversityGame/Blueprints/Characters/ActorParent.ActorParent_C|SetStateTeacher _array_element "NewEnumerator2"))
  (UserInterface|Viewport|AddtoPlayerScreen _returnvalue)
  (Rendering|SetVisibility (Variables|Default|GetStaticMesh) false false)
  (CallFunction|IncrementRecord)
  (Utilities|FlowControl|Delay 2.0)
  (Widget|RemovefromParent _returnvalue)
  (Actor|DestroyActor))

(event EventBeginPlay)

(event Collision|EventActorBeginOverlap
  (params (OtherActor :type Actor%20Object%20Reference)))

(fn ConstructionScript
  (|CallParentFunction))

(fn UseObject
  (bind _used_ (|CallParentFunction))
  (return _used_))