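; Laptop pickup that triggers when its box is overlapped, destroying the box so it fires only once.
; It shows a pickup banner, switches every Student_Jesus and Actor_JuanPedro to a new StateTeacher and reveals their cylinder and sphere meshes.
; It then hides itself, opens the Computer widget with UI-only input and player input disabled, and increments a record.
; After a short delay it removes the banner and destroys itself.
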(event OnComponentBeginOverlap(Box)
  (params (OverlappedComponent :type Primitive%20Component%20Object%20Reference) (OtherActor :type Actor%20Object%20Reference) (OtherComp :type Primitive%20Component%20Object%20Reference) (OtherBodyIndex :type Integer) (bFromSweep :type Boolean) (SweepResult :type Hit%20Result%20Structure%20%28by%20ref%29))
  (bind _returnvalue (Game|GetPlayerController 0))
  (Components|DestroyComponent (Variables|Default|GetBox))
  (bind _asmain_actor (Utilities|Casting|CastToMainActor (Game|GetPlayerCharacter 0)))
  (Variables|/Game/UniversityGame/Blueprints/Characters/MainActor.MainActor_C|SetBanner _asmain_actor "¡Has cogido el portátil!")
  (bind _returnvalue_2 (UserInterface|CreateWidget "/Game/UniversityGame/Blueprints/Widgets/Banner.Banner_C" (Game|GetPlayerController 0)))
  (UserInterface|Viewport|AddtoPlayerScreen _returnvalue_2)
  (Utilities|Casting|CastToGameInstanceUniversity (Game|GetGameInstance))
  (bind _outactors (Actor|GetAllActorsOfClass "/Game/UniversityGame/Blueprints/Characters/Student_Jesus.Student_Jesus_C"))
  (for _array_element _outactors
    (Variables|/Game/UniversityGame/Blueprints/Characters/ActorParent.ActorParent_C|SetStateTeacher _array_element "NewEnumerator2")
    (Rendering|SetVisibility (Variables|/Game/UniversityGame/Blueprints/Characters/ActorParent.ActorParent_C|GetCylinder _array_element) true false))
  (bind _outactors_2 (Actor|GetAllActorsOfClass "/Game/UniversityGame/Blueprints/Characters/Actor_JuanPedro.Actor_JuanPedro_C"))
  (for _array_element_2 _outactors_2
    (Variables|/Game/UniversityGame/Blueprints/Characters/ActorParent.ActorParent_C|SetStateTeacher _array_element_2 "NewEnumerator2")
    (Rendering|SetVisibility (Variables|/Game/UniversityGame/Blueprints/Characters/ActorParent.ActorParent_C|GetCylinder _array_element_2) true false))
  (Rendering|SetVisibility (Variables|Default|GetStaticMesh) false false)
  (bind _returnvalue_3 (UserInterface|CreateWidget "/Game/UniversityGame/Blueprints/Widgets/Computer.Computer_C"))
  (UserInterface|Viewport|AddtoPlayerScreen _returnvalue_3)
  (Input|SetInputModeUIOnly _returnvalue _returnvalue_3 "DoNotLock")
  (Variables|/Script/Engine.PlayerController|SetbShowMouseCursor _returnvalue true)
  (Input|DisableInput (Game|GetPlayerCharacter 0) _returnvalue)
  (CallFunction|IncrementRecord)
  (Utilities|FlowControl|Delay 2.0)
  (Widget|RemovefromParent _returnvalue_2)
  (Actor|DestroyActor))

(event EventBeginPlay)

(event Collision|EventActorBeginOverlap
  (params (OtherActor :type Actor%20Object%20Reference)))

(fn ConstructionScript
  (|CallParentFunction))

(fn UseObject
  (bind _used_ (|CallParentFunction))
  (return _used_))