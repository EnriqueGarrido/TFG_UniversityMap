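; Weapon pickup actor that attaches to the player character when its Box trigger registers an overlap, without checking which actor overlapped.
; The Weapon component snaps to the "Weapon" socket on player 0's character mesh.
; It then sets MainActor's Banner text to a Spanish pickup message and shows a Banner widget.
; After a short delay it removes the widget and destroys the Box, ending further pickups.
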(event OnComponentBeginOverlap(Box)
  (params (OverlappedComponent :type Primitive%20Component%20Object%20Reference) (OtherActor :type Actor%20Object%20Reference) (OtherComp :type Primitive%20Component%20Object%20Reference) (OtherBodyIndex :type Integer) (bFromSweep :type Boolean) (SweepResult :type Hit%20Result%20Structure%20%28by%20ref%29))
  ;[1 1 1] Change variable key
  (Transformation|AttachComponentToComponent (Variables|Default|GetWeapon) (Variables|/Script/Engine.Character|GetMesh (Game|GetPlayerCharacter 0)) "Weapon" "SnapToTarget" "SnapToTarget" "SnapToTarget" true)
  (bind _asmain_actor (Utilities|Casting|CastToMainActor (Game|GetPlayerCharacter 0)))
  (Variables|/Game/UniversityGame/Blueprints/Characters/MainActor.MainActor_C|SetBanner _asmain_actor "¡Has cogido el arma!")
  (bind _returnvalue (UserInterface|CreateWidget "/Game/UniversityGame/Blueprints/Widgets/Banner.Banner_C" (Game|GetPlayerController 0)))
  (UserInterface|Viewport|AddtoPlayerScreen _returnvalue)
  (Utilities|FlowControl|Delay 2.0)
  (Widget|RemovefromParent _returnvalue)
  (Components|DestroyComponent (Variables|Default|GetBox)))

(event EventBeginPlay)

(event Collision|EventActorBeginOverlap
  (params (OtherActor :type Actor%20Object%20Reference)))

(event EventTick
  (params (DeltaSeconds :type Float%20%28single-precision%29)))

(fn ConstructionScript)