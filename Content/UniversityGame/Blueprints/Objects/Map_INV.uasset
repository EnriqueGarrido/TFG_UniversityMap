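; Minimap pickup actor that grants the player the map when something overlaps its box trigger.
; The trigger destroys itself, sets HasMap on MainActor, and updates Actor_Ramon by revealing its cylinder and sphere and changing its teacher state.
; It then shows a Spanish pickup banner, hides the mesh, increments a record, and removes banner and actor after a short delay.
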(event OnComponentBeginOverlap(Box)
  (params (OverlappedComponent :type Primitive%20Component%20Object%20Reference) (OtherActor :type Actor%20Object%20Reference) (OtherComp :type Primitive%20Component%20Object%20Reference) (OtherBodyIndex :type Integer) (bFromSweep :type Boolean) (SweepResult :type Hit%20Result%20Structure%20%28by%20ref%29))
  ;[1 1 1] You have the minimap
  (Components|DestroyComponent (Variables|Default|GetBox))
  (bind _asmain_actor (Utilities|Casting|CastToMainActor (Game|GetPlayerCharacter 0)))
  (Variables|/Game/UniversityGame/Blueprints/Characters/MainActor.MainActor_C|SethasMap _asmain_actor true)
  (bind _outactors (Actor|GetAllActorsOfClass "/Game/UniversityGame/Blueprints/Characters/Actor_Ramon.Actor_Ramon_C"))
  (for _array_element _outactors
    (bind _output_get (Variables|Default|SetActorRamon _array_element)))
  (Rendering|SetVisibility (Variables|/Game/UniversityGame/Blueprints/Characters/ActorParent.ActorParent_C|GetCylinder _output_get) true false)
  (Rendering|SetVisibility (Variables|/Game/UniversityGame/Blueprints/Characters/ActorParent.ActorParent_C|GetSphere _output_get) true false)
  (Variables|/Game/UniversityGame/Blueprints/Characters/ActorParent.ActorParent_C|SetStateTeacher _output_get "NewEnumerator2")
  (bind _asmain_actor_2 (Utilities|Casting|CastToMainActor (Game|GetPlayerCharacter 0)))
  (Variables|/Game/UniversityGame/Blueprints/Characters/MainActor.MainActor_C|SetBanner _asmain_actor_2 "¡Has cogido el minimapa!")
  (bind _returnvalue (UserInterface|CreateWidget "/Game/UniversityGame/Blueprints/Widgets/Banner.Banner_C" (Game|GetPlayerController 0)))
  (UserInterface|Viewport|AddtoPlayerScreen _returnvalue)
  (Rendering|SetVisibility (Variables|Default|GetStaticMesh) false false)
  (CallFunction|IncrementRecord)
  (Utilities|FlowControl|Delay 2.0)
  (Widget|RemovefromParent _returnvalue)
  (Actor|DestroyActor))

(fn ConstructionScript
  (|CallParentFunction))