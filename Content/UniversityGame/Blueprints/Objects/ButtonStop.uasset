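; ButtonStop is an interactable button that wipes out every RobotEnemy in the level.
; Overlapping its Box shows a text prompt and enables player input, and leaving hides the prompt and disables input.
; Pressing O while input is enabled destroys all RobotEnemy actors, then sets HasSpawnedRobot to true on the player's MainActor character.
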(event OnComponentBeginOverlap(Box)
  (params (OverlappedComponent :type Primitive%20Component%20Object%20Reference) (OtherActor :type Actor%20Object%20Reference) (OtherComp :type Primitive%20Component%20Object%20Reference) (OtherBodyIndex :type Integer) (bFromSweep :type Boolean) (SweepResult :type Hit%20Result%20Structure%20%28by%20ref%29))
  ;[1 1 1] Appear or desappear box
  (Rendering|SetVisibility (Variables|Default|GetTextRender) true false)
  (Input|EnableInput (Game|GetPlayerController 0)))

(event OnComponentEndOverlap(Box)
  (params (OverlappedComponent :type Primitive%20Component%20Object%20Reference) (OtherActor :type Actor%20Object%20Reference) (OtherComp :type Primitive%20Component%20Object%20Reference) (OtherBodyIndex :type Integer))
  ;[1 1 1] Appear or desappear box
  (Rendering|SetVisibility (Variables|Default|GetTextRender) false false)
  (Input|DisableInput (Game|GetPlayerController 0)))

(event EventBeginPlay
  ;[1 1 1] Event beginplay
  (Rendering|SetVisibility (Variables|Default|GetTextRender) false false)
  (Variables|Default|SetRotation (Transformation|GetActorRotation)))

(event Input|KeyboardEvents|O
  (params (Key :type Key%20Structure))
  ;[1 1 1] Eliminate all robots
  (:Pressed
    (bind _outactors (Actor|GetAllActorsOfClass "/Game/UniversityGame/Blueprints/IAEnemy/RobotEnemy.RobotEnemy_C"))
    (for _array_element _outactors
      (Actor|DestroyActor _array_element))
    (bind _asmain_actor (Utilities|Casting|CastToMainActor (Game|GetPlayerCharacter 0)))
    (Variables|/Game/UniversityGame/Blueprints/Characters/MainActor.MainActor_C|SethasSpawnedRobot _asmain_actor true)))

(fn ConstructionScript)