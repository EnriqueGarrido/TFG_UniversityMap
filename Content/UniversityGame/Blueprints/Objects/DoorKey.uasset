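; DoorKey is a locked door that the player toggles open and closed by yaw rotation, requiring a key and not being zombie-blocked.
; A box overlap shows prompt texts and enables input for the OpenDoor action, which checks the MainActor's HasKeyDoor flag.
; On first use, it removes the key from the inventory through InventoryWindow and Spaces widgets, then briefly shows a Banner, with WidgetActivated preventing repeats.
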(event OnComponentBeginOverlap(Box)
  (params (OverlappedComponent :type Primitive%20Component%20Object%20Reference) (OtherActor :type Actor%20Object%20Reference) (OtherComp :type Primitive%20Component%20Object%20Reference) (OtherBodyIndex :type Integer) (bFromSweep :type Boolean) (SweepResult :type Hit%20Result%20Structure%20%28by%20ref%29))
  ;[1 1 1] Appear or desappear box
  (Rendering|SetVisibility (Variables|Default|GetTextRender) true false)
  (Input|EnableInput (Game|GetPlayerController 0)))

(event OnComponentEndOverlap(Box)
  (params (OverlappedComponent :type Primitive%20Component%20Object%20Reference) (OtherActor :type Actor%20Object%20Reference) (OtherComp :type Primitive%20Component%20Object%20Reference) (OtherBodyIndex :type Integer))
  ;[1 1 1] Appear or desappear box
  (Rendering|SetVisibility (Variables|Default|GetTextRender) false false)
  (Input|DisableInput (Game|GetPlayerController 0)))

(event EventBeginPlay
  ;[1 1 1] Event beginplay
  (Rendering|SetVisibility (Variables|Default|GetTextRender) false false)
  (Variables|Default|SetRotation (Transformation|GetActorRotation)))

(event Input|ActionEvents|InputActionOpenDoor
  (params (Key :type Key%20Structure))
  (bind _returnvalue (Game|GetPlayerController 0))
  (bind _rotation (Variables|Default|GetRotation))
  (bind (_roll _pitch _yaw) (Math|Rotator|BreakRotator _rotation))
  ;[1 1 1] Open or Close when you has key
  (:Pressed
    (if (not (Variables|Default|GetZombiesBlocked))
      (bind _asmain_actor (Utilities|Casting|CastToMainActor (Game|GetPlayerCharacter 0)))
      (if (Variables|/Game/UniversityGame/Blueprints/Characters/MainActor.MainActor_C|GethasKeyDoor _asmain_actor)
        (if (Variables|Default|GetWidgetActivated)
          _
          (else
            (bind _asmain_actor_2 (Utilities|Casting|CastToMainActor (Game|GetPlayerCharacter 0)))
            (bind _returnvalue_2 (UserInterface|CreateWidget "/Game/UniversityGame/Blueprints/Widgets/InventoryWindow.InventoryWindow_C" _returnvalue (Variables|/Game/UniversityGame/Blueprints/Characters/MainActor.MainActor_C|GetInvent_Component _asmain_actor_2)))
            (bind (_container _index) (Default|FindSpace _returnvalue_2 "Key"))
            (bind _returnvalue_3 (UserInterface|CreateWidget "/Game/UniversityGame/Blueprints/Widgets/sPACES.Spaces_C" _returnvalue _index _container (Variables|/Game/UniversityGame/Blueprints/Characters/MainActor.MainActor_C|GetInvent_Component _asmain_actor_2)))
            (Default|Eliminate _returnvalue_3 _container _index)
            (bind _asmain_actor_3 (Utilities|Casting|CastToMainActor (Game|GetPlayerCharacter 0)))
            (Variables|/Game/UniversityGame/Blueprints/Characters/MainActor.MainActor_C|SetBanner _asmain_actor_3 "¡Has usado una llave para abrir la puerta!")))
        (if (Variables|Default|GetDoorOpen)
          (Transformation|SetActorRotation (Variables|Default|GetRotation))
          (Variables|Default|SetDoorOpen false)
          (else
            (Transformation|SetActorRotation (Math|Rotator|MakeRotator _roll _pitch (- _yaw 9e+01)))
            (Variables|Default|SetDoorOpen true)))
        (if (not (Variables|Default|GetWidgetActivated))
          (Variables|Default|SetWidgetActivated true)
          (bind _returnvalue_4 (UserInterface|CreateWidget "/Game/UniversityGame/Blueprints/Widgets/Banner.Banner_C" (Game|GetPlayerController 0)))
          (UserInterface|Viewport|AddtoPlayerScreen _returnvalue_4)
          (Utilities|FlowControl|Delay 2.0)
          (Widget|RemovefromParent _returnvalue_4))))))

(fn ConstructionScript)